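; BP_Lighting switches a level between day and night lighting based on its Night flag.
; ToggleLighting stores the flag, then shows or hides the day actors (height fog, lights, sky base, post-process volume) and sets the night lighting root's visibility to the opposite state.
; Both the construction script and BeginPlay apply the flag, so the chosen state previews in the editor and holds at runtime.
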(event Custom|SetDayVisability
  (params (Visable :type Boolean))
  (Utilities|FlowControl|Sequence
    (:then_0
      (Rendering|SetVisibility (Variables|/Script/Engine.ExponentialHeightFog|GetComponent (Variables|Day|GetDay_EHF)) Visable true))
    (:then_1
      (Rendering|SetVisibility (Variables|/Script/Engine.Light|GetLightComponent (Variables|Day|GetDay_LS)) Visable true))
    (:then_2
      (Variables|/Script/Engine.PostProcessVolume|SetbEnabled (Variables|Day|GetDay_PPV) Visable))
    (:then_3
      (Rendering|SetVisibility (Variables|/Script/Engine.SkyLight|GetLightComponent (Variables|Day|GetDay_SL)) Visable true))
    (:then_4
      (Rendering|SetVisibility (Variables|/Engine/EngineSky/BP_Sky_Sphere.BP_Sky_Sphere_C|GetBase (Variables|Day|GetDay_SSB)) Visable true))))

(event Custom|SetNightVisability
  (params (Visability :type Boolean))
  (Rendering|SetVisibility (Variables|/Game/LightingNightTime.LightingNightTime_C|GetSharedRoot (Variables|Night|GetNight_Lighting)) Visability true))

(event Custom|ToggleLighting
  (params (Night :type Boolean))
  (bind _output_get (Variables|Default|SetNight Night))
  (CallFunction|SetDayVisability (not _output_get))
  (CallFunction|SetNightVisability _output_get))

(event EventBeginPlay
  (CallFunction|ToggleLighting (Variables|Default|GetNight)))

(fn ConstructionScript
  (CallFunction|ToggleLighting (Variables|Default|GetNight)))