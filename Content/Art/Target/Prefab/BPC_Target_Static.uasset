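; Static shooting-target Blueprint that starts folded down, pops up when shown, wobbles when hit and falls when out of health.
; Show plays a timeline that raises the mesh and enables hit reactions.
; Hit scales a timeline wobble by the incoming Dot value, checking health before and after it to trigger the fall and mark it dead.
; CurrentHP starts at MaxHP but is never reduced here.
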(event Custom|Hit
  (params (Dot :type Float%20%28single-precision%29%20%28by%20ref%29))
  (bind _currenthp (Variables|Default|GetCurrentHP))
  (bind _returnvalue (<= _currenthp 0.0))
  (if (Variables|Default|GetShowing)
    (if (not (Variables|Default|GetDead))
      (if _returnvalue
        (Variables|Default|SetDead true :!label _label)
        (Components|Timeline|SetPlayRate (Variables|Default|GetTimeline_1) 0.8)
        (bind _fall (Timeline|Timeline_1 PlayFromStart)
          (:Update
            (Transformation|SetRelativeRotation (Variables|Default|GetSM_Target_Static_Static_01) (Math|Rotator|Lerp(Rotator) "0, 0, 0" "0, 0,-92.000000" _fall) false false)))
        (else
          (bind _hit (Timeline|Timeline_0 PlayFromStart)
            (:Update
              (Transformation|SetRelativeRotation (Variables|Default|GetSM_Target_Static_Static_01) (Class|KismetMathLibrary|QuatRotator (Class|KismetMathLibrary|QuatMakefromEuler (Math|Vector|MakeVector (* _hit (* Dot 5.0)) 0.0 0.0))) false false))
            (:Finished
              (if _returnvalue
                (goto _label)))))))))

(event Custom|Show
  (if (not (Variables|Default|GetShowing))
    (Components|Timeline|SetPlayRate (Variables|Default|GetShowGraph) 1.5)
    (bind _newtrack_0 (Timeline|ShowGraph Play)
      (:Update
        (Transformation|SetRelativeRotation (Variables|Default|GetSM_Target_Static_Static_01) (Math|Rotator|Lerp(Rotator) "0, 0,-92.000000" "0, 0,0.000000" _newtrack_0) false false))
      (:Finished
        (Variables|Default|SetShowing true)))))

(event EventBeginPlay
  (Variables|Default|SetCurrentHP (Variables|Default|GetMaxHP))
  (Transformation|SetRelativeRotation (Variables|Default|GetSM_Target_Static_Static_01) "0, 0,-92.000000" false false))

(event Collision|EventActorBeginOverlap
  (params (OtherActor :type Actor%20Object%20Reference)))

(event EventTick
  (params (DeltaSeconds :type Float%20%28single-precision%29)))

(fn ConstructionScript)