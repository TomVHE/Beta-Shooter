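; Moving target that slides back and forth between two points and reacts to hits until it falls over.
; A looping timeline, paced by Timing and started in a random direction, lerps the base between StartPoint and EndPoint, stopping once Dead.
; Hit plays a wobble scaled by the incoming Dot, or a fall timeline when HP is depleted.
; CurrentHP starts at MaxHP and is only checked here, never decremented.
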(event Custom|Hit
  (params (Dot :type Float%20%28single-precision%29%20%28by%20ref%29))
  (bind _sm_target_dynamic_dynamic_01 (Variables|Default|GetSM_Target_Dynamic_Dynamic_01))
  (bind _currenthp (Variables|Default|GetCurrentHP))
  (bind _returnvalue (<= _currenthp 0.0))
  (if (not (Variables|Default|GetDead))
    (if _returnvalue
      (Variables|Default|SetDead true :!label _label)
      (bind _fall (Timeline|Timeline_1 PlayFromStart)
        (:Update
          (Transformation|SetRelativeRotation _sm_target_dynamic_dynamic_01 (Math|Rotator|Lerp(Rotator) (Variables|/Script/Engine.SceneComponent|GetRelativeRotation _sm_target_dynamic_dynamic_01) "0, 0,-92.000000" _fall) false false)))
      (else
        (bind _hit (Timeline|Timeline_0 PlayFromStart)
          (:Update
            (Transformation|SetRelativeRotation _sm_target_dynamic_dynamic_01 (Class|KismetMathLibrary|QuatRotator (Class|KismetMathLibrary|QuatMakefromEuler (Math|Vector|MakeVector (* _hit (* Dot 5.0)) 0.0 0.0))) false false))
          (:Finished
            (if _returnvalue
              (goto _label))))))))

(event EventBeginPlay
  (Variables|Default|SetCurrentHP (Variables|Default|GetMaxHP))
  (Variables|Default|SetReverse (Math|Random|RandomBool))
  (Components|Timeline|SetPlayRate (Variables|Default|GetTimeline_2) (/ 1.0 (Variables|Default|GetTiming)))
  (if (Variables|Default|GetReverse) :!label _label
    (bind _float (Timeline|Timeline_2 ReverseFromEnd)
      (:Update
        (Transformation|SetRelativeLocation (Variables|Default|GetSM_Target_Dynamic_Base_Dynamic_01) (Math|Vector|Lerp(Vector) (Variables|Default|GetStartPoint) (Variables|Default|GetEndPoint) _float) false false)
        (if (Variables|Default|GetDead)
          (Timeline|Timeline_2 Stop)))
      (:Finished
        (Variables|Default|SetReverse (>= _float 1.0))
        (goto _label)))
    (else
      (Timeline|Timeline_2 PlayFromStart))))

(event Collision|EventActorBeginOverlap
  (params (OtherActor :type Actor%20Object%20Reference)))

(event EventTick
  (params (DeltaSeconds :type Float%20%28single-precision%29)))

(fn ConstructionScript)