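; Dynamic shooting target that registers with SectionsManager by section, starts folded down at a random end of its track, and pops up on Show.
; Once up, it shuttles between StartPoint and EndPoint on a looping timeline paced by Timing.
; Hits play a wobble scaled by Dot; when CurrentHP, which is not reduced here, is depleted, it unregisters, falls flat and stops moving.
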(event Custom|Hit
  (params (Dot :type Float%20%28single-precision%29%20%28by%20ref%29))
  (bind _sm_target_dynamic_dynamic_01 (Variables|Default|GetSM_Target_Dynamic_Dynamic_01))
  (bind _currenthp (Variables|Default|GetCurrentHP))
  (bind _returnvalue (<= _currenthp 0.0))
  (if (Variables|Default|GetShowing)
    (if (not (Variables|Default|GetDead))
      (if _returnvalue
        (Variables|Default|SetDead true :!label _label)
        (Default|RemoveDynamicTarget (Variables|Default|GetSectionsManager) (Variables|Default|GetSection) self)
        (Components|Timeline|SetPlayRate (Variables|Default|GetTimeline_1) 0.8)
        (bind _fall (Timeline|Timeline_1 PlayFromStart)
          (:Update
            (Transformation|SetRelativeRotation _sm_target_dynamic_dynamic_01 (Math|Rotator|Lerp(Rotator) "0, 0, 0" "0, 0,-92.000000" _fall) false false)))
        (else
          (bind _hit (Timeline|Timeline_0 PlayFromStart)
            (:Update
              (Transformation|SetRelativeRotation _sm_target_dynamic_dynamic_01 (Class|KismetMathLibrary|QuatRotator (Class|KismetMathLibrary|QuatMakefromEuler (Math|Vector|MakeVector (* _hit (* Dot 5.0)) 0.0 0.0))) false false))
            (:Finished
              (if _returnvalue
                (goto _label)))))))))

(event Custom|Show
  (if (not (Variables|Default|GetShowing))
    (Components|Timeline|SetPlayRate (Variables|Default|GetShowGraph) 1.5)
    (bind _newtrack_0 (Timeline|ShowGraph PlayFromStart)
      (:Update
        (Transformation|SetRelativeRotation (Variables|Default|GetSM_Target_Dynamic_Dynamic_01) (Math|Rotator|Lerp(Rotator) "0, 0,-92.000000" "0, 0, 0" _newtrack_0) false false))
      (:Finished
        (Variables|Default|SetShowing true)
        (Components|Timeline|SetPlayRate (Variables|Default|GetTimeline_2) (/ 1.0 (Variables|Default|GetTiming)))
        (if (Variables|Default|GetReverse) :!label _label
          (bind _float (Timeline|Timeline_2 ReverseFromEnd)
            (:Update
              (Transformation|SetRelativeLocation (Variables|Default|GetSM_Target_Dynamic_Base_Dynamic_01) (Math|Vector|Lerp(Vector) (Variables|Default|GetStartPoint) (Variables|Default|GetEndPoint) _float) false false)
              (if (Variables|Default|GetDead)
                (Timeline|Timeline_2 Stop)))
            (:Finished
              (Variables|Default|SetReverse (>= _float 1.0))
              (goto _label)))
          (else
            (Timeline|Timeline_2 PlayFromStart)))))))

(event EventBeginPlay
  (bind _sm_target_dynamic_base_dynamic_01 (Variables|Default|GetSM_Target_Dynamic_Base_Dynamic_01))
  (Default|AddDynamicTarget (Variables|Default|GetSectionsManager) (Variables|Default|GetSection) self)
  (Variables|Default|SetCurrentHP (Variables|Default|GetMaxHP))
  (bind _output_get (Variables|Default|SetReverse (Math|Random|RandomBool)))
  (if _output_get
    (Transformation|SetRelativeLocation _sm_target_dynamic_base_dynamic_01 (Variables|Default|GetEndPoint) false false)
    (else
      (Transformation|SetRelativeLocation _sm_target_dynamic_base_dynamic_01 (Variables|Default|GetStartPoint) false false)))
  (Transformation|SetRelativeRotation (Variables|Default|GetSM_Target_Dynamic_Dynamic_01) "0, 0,-92.000000" false false))

(fn ConstructionScript)