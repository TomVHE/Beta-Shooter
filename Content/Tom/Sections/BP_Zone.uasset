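; BP_Zone is a trigger zone for a timed target challenge, identified by section and zone index.
; When Player_Test first overlaps it with CanShow set, it shows its Targets, zeroes score and kills, and starts a looping 0.1-second timer.
; Each KilledTarget call adds score and updates BP_SectionManager; the last kill stops the timer and reports completion.
; Reset hides all targets but leaves CanShow untouched.
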(event Custom|KilledTarget
  (params (Score :type Integer%20%28by%20ref%29))
  (Variables|Default|SetScore (+ Score (Variables|Default|GetScore)))
  (bind _result (Math|Integer|IncrementInt (Variables|Default|GetKilled))
    (:%20%20
      (if (== _result (Utilities|Array|Length (Variables|Default|GetTargets)))
        (Utilities|Time|ClearandInvalidateTimerbyHandle (stale Collision|EventActorBeginOverlap _returnvalue))
        (bind _outactors (Actor|GetAllActorsOfClass "/Game/Tom/Sections/BP_SectionManager.BP_SectionManager_C"))
        (for _array_element _outactors
          (Default|CompletedZone _array_element (Variables|Default|GetSectionIndex) (Variables|Default|GetZoneIndex) (Utilities|Struct|MakeBP_Scoring (Variables|Default|GetScore) (Variables|Default|GetTime))))
        (else
          (bind _outactors_2 (Actor|GetAllActorsOfClass "/Game/Tom/Sections/BP_SectionManager.BP_SectionManager_C"))
          (Default|UpdateZone (Utilities|Array|Get(acopy) _outactors_2) (Variables|Default|GetSectionIndex) (Variables|Default|GetZoneIndex) (Utilities|Struct|MakeBP_Scoring (Variables|Default|GetScore) (Variables|Default|GetTime))))))))

(event Custom|Reset
  (for _array_element (Variables|Default|GetTargets)
    (Default|Hide _array_element true)))

(event EventBeginPlay
  (for _array_element (Variables|Default|GetTargets)
    (Variables|/Game/Tom/Targets/BP_Target.BP_Target_C|SetZone _array_element self)))

(event Collision|EventActorBeginOverlap
  (params (OtherActor :type Actor%20Object%20Reference))
  (if (Variables|Default|GetCanShow)
    (Utilities|Casting|CastToPlayer_Test OtherActor)
    (for _array_element (Variables|Default|GetTargets)
      (Default|Show _array_element))
    (Variables|Default|SetCanShow false)
    (Variables|Default|SetKilled 0)
    (Variables|Default|SetScore 0)
    (Variables|Default|SetTime 0.0)
    (bind _returnvalue (Utilities|Time|SetTimerbyFunctionName self "UpdateTime" 0.1 true))))

(fn ConstructionScript)

(fn UpdateTime
  (Variables|Default|SetTime (+ (Variables|Default|GetTime) 0.1)))