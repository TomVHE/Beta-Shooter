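; Game manager Blueprint that wires up the section trigger zones, currently as an early scaffold with debug prints.
; On BeginPlay it loops over Section0 and binds each element's Collider overlap to ZoneTriggered_0, which only prints a message.
; Loops over each element's dynamic and static targets print placeholders for future collider retrieval.
; NewMacro_0 drafts the same nested iteration and outputs the Collider, while NewMacro_1 and the construction script are empty.
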(event Custom|ZoneTriggered_0
  (params (OverlappedActor :type Actor%20Object%20Reference) (OtherActor :type Actor%20Object%20Reference))
  (Development|PrintString "Zone Triggered"))

(event EventBeginPlay
  (for _array_element (Variables|Section0|GetSection_0)
    (EventDispatchers|AssignOnActorBeginOverlap (.Collider (Utilities|Struct|BreakZone _array_element)) (delegate Custom|ZoneTriggered_0))
    (for _array_element_2 (.Targets_Dynamic (Utilities|Struct|BreakZone _array_element))
      (Development|PrintString "Get collider of dynamic target here"))
    (for _array_element_3 (.Targets_Static (Utilities|Struct|BreakZone _array_element))
      (Development|PrintString "Get collider of static target here"))))

(fn ConstructionScript)