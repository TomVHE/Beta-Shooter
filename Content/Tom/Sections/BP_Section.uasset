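; BP_Section reveals groups of targets when the player enters trigger zones within a level section.
; BeginPlay binds overlap events on trigger boxes in three zone arrays, using nested loops.
; When a Player_Test overlaps a box, GetZone searches each array in turn for the matching collider.
; ShowTargets then calls Show on that zone's dynamic and static targets.
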(event Custom|ZoneOverlap
  (params (OverlappedActor :type Actor%20Object%20Reference) (OtherActor :type Actor%20Object%20Reference))
  (bind _zones_0 (Variables|Section0|GetZones_0))
  (bind _zones_1 (Variables|Section1|GetZones_1))
  (bind _zones_2 (Variables|Section2|GetZones_2))
  (Utilities|Casting|CastToPlayer_Test OtherActor)
  (bind _astrigger_box (Utilities|Casting|CastToTriggerBox OverlappedActor))
  (bind _index (Utilities|GetZone _astrigger_box _zones_0)
    (:True
      (Utilities|ShowTargets _zones_0 _index))
    (:False
      (bind _index_2 (Utilities|GetZone _astrigger_box _zones_1)
        (:True
          (Utilities|ShowTargets _zones_1 _index_2))
        (:False
          (bind _index_3 (Utilities|GetZone _astrigger_box _zones_2)
            (:True
              (Utilities|ShowTargets _zones_2 _index_3))))))))

(event EventBeginPlay
  (for _array_element (Variables|Section0|GetZones_0)
    (EventDispatchers|AssignOnActorBeginOverlap (Utilities|Struct|BreakZone _array_element) (delegate Custom|ZoneOverlap))
    (for _array_element_2 (Variables|Section1|GetZones_1)
      (EventDispatchers|AssignOnActorBeginOverlap (.Collider (Utilities|Struct|BreakZone _array_element_2)) (delegate Custom|ZoneOverlap))
      (for _array_element_3 (Variables|Section2|GetZones_2)
        (EventDispatchers|AssignOnActorBeginOverlap (.Collider (Utilities|Struct|BreakZone _array_element_3)) (delegate Custom|ZoneOverlap))))))

(fn ConstructionScript)

(fn BPSectionAutoGenFunc
  (params (OverlappedActor :type Actor%20Object%20Reference) (OtherActor :type Actor%20Object%20Reference)))