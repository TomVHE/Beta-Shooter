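; Sideways variant of a shooting target that swings on a hinge to show, hide and react to hits.
; Show and Hide drive timelines scaled by rise and fall times, lerping the hinge between zero and DownRotator, while an instant Hide snaps it to zero.
; Show also restores health and makes the target hittable once the swing finishes.
; HitAnim maps an incoming value to a slight wobble around DownRotator.
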(event EventBeginPlay
  (|CallParentFunction) ; This node is disabled and will not be called.\nDrag off pins to build functionality.
)

(event EventHitAnim
  (params (Value :type Float%20%28single-precision%29))
  (Transformation|SetRelativeRotation (Variables|Default|GetTargetHinge) (Math|Rotator|Lerp(Rotator) (Math|Rotator|CombineRotators (Variables|Default|GetDownRotator) "0.500000, 0, 0") (Math|Rotator|CombineRotators (Variables|Default|GetDownRotator) "-0.500000, 0, 0") Value) false false))

(event EventHide
  (params (Instant :type Boolean))
  (if Instant
    (Transformation|SetRelativeRotation (Variables|Default|GetTargetHinge) "0, 0, 0" false false)
    (else
      (Components|Timeline|SetPlayRate (Variables|Default|GetTimeline_0) (/ 1.0 (Variables|Default|GetFallTime)))
      (bind _value (Timeline|Timeline_0 PlayFromStart)
        (:Update
          (Transformation|SetRelativeRotation (Variables|Default|GetTargetHinge) (Math|Rotator|Lerp(Rotator) (Variables|Default|GetDownRotator) "0, 0, 0" _value true) false false))))))

(event EventShow
  (Variables|Default|SetCurrentHealth (Variables|Default|GetHealth))
  (Components|Timeline|SetPlayRate (Variables|Default|GetTimeline_1) (/ 1.0 (Variables|Default|GetRiseTime)))
  (bind _value (Timeline|Timeline_1 PlayFromStart)
    (:Update
      (Transformation|SetRelativeRotation (Variables|Default|GetTargetHinge) (Math|Rotator|Lerp(Rotator) "0, 0, 0" (Variables|Default|GetDownRotator) _value true) false false))
    (:Finished
      (Variables|Default|SetHitable true))))

(fn ConstructionScript
  (|CallParentFunction))