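; Pop-up shooting target that starts folded down on its hinge and reports its score to its Zone when killed.
; Show resets health and score, then raises the target by timeline, making it hittable once upright.
; Hit always attaches a bullet decal; while hittable, it scores head above body and subtracts damage.
; Timelines drive a brief wobble on non-lethal hits and the fall at zero health, with playback rates derived from durations.
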(event Custom|Hide
  (params (Instant :type Boolean))
  (if Instant
    (Transformation|SetRelativeRotation (Variables|Default|GetTargetHinge) (Variables|Default|GetDownRotator) false false)
    (else
      (Components|Timeline|SetPlayRate (Variables|Default|GetTL_Fall) (/ 1.0 (Variables|Default|GetFallTime)))
      (bind _value (Timeline|TL_Fall PlayFromStart)
        (:Update
          (Transformation|SetRelativeRotation (Variables|Default|GetTargetHinge) (Math|Rotator|Lerp(Rotator) "0, 0, 0" (Variables|Default|GetDownRotator) _value true) false false))))))

(event Custom|Show
  (Variables|Default|SetCurrentHealth (Variables|Default|GetHealth))
  (Variables|Default|SetScore 0)
  (Components|Timeline|SetPlayRate (Variables|Default|GetTL_Rise) (/ 1.0 (Variables|Default|GetRiseTime)))
  (bind _value (Timeline|TL_Rise PlayFromStart)
    (:Update
      (Transformation|SetRelativeRotation (Variables|Default|GetTargetHinge) (Math|Rotator|Lerp(Rotator) (Variables|Default|GetDownRotator) "0, 0, 0" _value true) false false))
    (:Finished
      (Variables|Default|SetHitable true))))

(event Custom|Hit
  (params (Component :type Primitive%20Component%20Object%20Reference) (Damage :type Float%20%28single-precision%29%20%28by%20ref%29) (Position :type Vector%20%28by%20ref%29))
  (bind _score (Variables|Default|GetScore))
  (bind _returnvalue (Class|GameplayStatics|SpawnDecalAttached "/Game/Art/Bullet_Decals/Bullet_Decal.Bullet_Decal" "5.000000,5.000000,5.000000" (Variables|Default|GetTargetPlank) "None" (Math|Transform|InverseTransformLocation (Transformation|GetWorldTransform (Variables|Default|GetTargetPlank)) Position) (Math|Rotator|MakeRotator (Math|Random|RandomFloatinRange -1.8e+02 1.8e+02) 0.0 2.7e+02) "SnapToTarget" 1e+01))
  (Rendering|Components|Decal|SetFadeScreenSize _returnvalue 0.001)
  (if (Variables|Default|GetHitable)
    (if (== Component (Variables|Default|GetHeadCollider))
      (Math|Integer|IncrementInt _score
        (:%20%20
          (Math|Integer|IncrementInt _score
            (:%20%20
              _))))
      (elif (== Component (Variables|Default|GetBodyCollider))
        (Math|Integer|IncrementInt _score
          (:%20%20
            _))))
    (bind _output_get (Variables|Default|SetCurrentHealth (- (Variables|Default|GetCurrentHealth) Damage)))
    (if (<= _output_get 0.0)
      (Variables|Default|SetHitable false)
      (CallFunction|Hide false)
      (Default|KilledTarget (Variables|Default|GetZone) (Variables|Default|GetScore))
      (else
        (Components|Timeline|SetPlayRate (Variables|Default|GetHitEffect) (/ 1.0 0.2))
        (bind _value (Timeline|HitEffect PlayFromStart)
          (:Update
            (CallFunction|HitAnim _value)))))))

(event Custom|HitAnim
  (params (Value :type Float%20%28single-precision%29))
  (Transformation|SetRelativeRotation (Variables|Default|GetTargetHinge) (Math|Rotator|Lerp(Rotator) "0, 0,0.500000" "0, 0,-0.500000" Value) false false))

(event EventBeginPlay
  (Variables|Default|SetDownRotator (Math|Rotator|MakeRotator (Variables|Default|GetDownRotation) 0.0 0.0))
  (CallFunction|Hide true)
  (Variables|Default|SetCurrentHealth (Variables|Default|GetHealth)))

(fn ConstructionScript)