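; BP_Target_Dynamic is a child target Blueprint whose TargetBase slides side to side while it is hittable.
; BeginPlay picks a random direction, places the base at the matching end and sets the Movement timeline rate to the inverse of MovementSpeed.
; Tick plays or reverses the timeline by direction, or stops it when Hitable is false.
; The timeline lerps the base's relative X between RightPosition and LeftPosition, flipping direction on finish.
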(event EventBeginPlay
  (bind _targetbase (Variables|Default|GetTargetBase))
  (bind _output_get (Variables|Default|SetPosA (Math|Vector|MakeVector (Variables|Default|GetRightPosition) 0.0 0.0)))
  (bind _output_get_2 (Variables|Default|SetPosB (Math|Vector|MakeVector (Variables|Default|GetLeftPosition) 0.0 0.0)))
  (bind _output_get_3 (Variables|Default|SetGoingLeft (Math|Random|RandomBool)))
  (if _output_get_3
    (Transformation|SetRelativeLocation _targetbase _output_get false false)
    (else
      (Transformation|SetRelativeLocation _targetbase _output_get_2 false false)))
  (Components|Timeline|SetPlayRate (Variables|Default|GetMovement) (/ 1.0 (Variables|Default|GetMovementSpeed)))
  (|CallParentFunction))

(event EventTick
  (params (DeltaSeconds :type Float%20%28single-precision%29))
  (if (Variables|Default|GetHitable)
    (if (Variables|Default|GetGoingLeft)
      (bind _newtrack_0 (Timeline|Movement Play)
        (:Update
          (Transformation|SetRelativeLocation (Variables|Default|GetTargetBase) (Math|Vector|Lerp(Vector) (Variables|Default|GetPosA) (Variables|Default|GetPosB) _newtrack_0) false false))
        (:Finished
          (Variables|Default|SetGoingLeft (not (Variables|Default|GetGoingLeft)))))
      (elif (== (Components|Timeline|GetPlaybackPosition (Variables|Default|GetMovement)) 0.0)
        (Timeline|Movement ReverseFromEnd)
        (else
          (Timeline|Movement Reverse))))
    (else
      (Timeline|Movement Stop))))

(fn ConstructionScript
  (|CallParentFunction))